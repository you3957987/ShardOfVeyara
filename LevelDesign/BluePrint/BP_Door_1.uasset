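; BP_Door_1 is an interactable double door that the player opens with the Interaction input and that closes when they leave.
; A Door_Ani timeline swings Door1 and Door2 90 degrees in opposite directions, playing from start to open and reversing to close.
; Any Box overlap enables player input on the door without a later disable, while only the player character leaving triggers the close.
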(event `DoorOpen`
  ; 문 열리는 애니메이션
  (bind (_direction `_새_트랙_0`) (`Timeline|Door_Ani` :!via `PlayFromStart` :!label _label)
    (:`Update`
      (`SceneComponent.K2_SetRelativeRotation` (`self.Door_1`) (`KismetMathLibrary.RLerp` (struct) (struct :`Yaw` 90.0) `_새_트랙_0` true) false false)
      (`SceneComponent.K2_SetRelativeRotation` (`self.Door_2`) (`KismetMathLibrary.RLerp` (struct) (struct :`Yaw` -90.0) `_새_트랙_0` true) false false))))

(event `DoorClose`
  ; 문 열리는 애니메이션
  (goto _label :!via `Reverse`))

(event `InputAction|Interaction`
  (params (Key :type "Key Structure"))
  ; 콜리젼 충돌 시 열고 닫힘
  (:`Pressed`
    (`self.DoorOpen`)))

(event `self.Box.OnComponentEndOverlap`
  (params (OverlappedComponent :type "PrimitiveComponent Object Reference") (OtherActor :type "Actor Object Reference") (OtherComp :type "PrimitiveComponent Object Reference") (OtherBodyIndex :type Integer))
  ; 콜리젼 충돌 시 열고 닫힘
  (if (== OtherActor (`GameplayStatics.GetPlayerCharacter` 0))
    (`self.DoorClose`)))

(event `self.Box.OnComponentBeginOverlap`
  (params (OverlappedComponent :type "PrimitiveComponent Object Reference") (OtherActor :type "Actor Object Reference") (OtherComp :type "PrimitiveComponent Object Reference") (OtherBodyIndex :type Integer) (bFromSweep :type Boolean) (SweepResult :type "HitResult Structure (by ref)"))
  ; 콜리젼 충돌 시 열고 닫힘
  (`self.EnableInput` (`GameplayStatics.GetPlayerController` 0)))

(fn `UserConstructionScript`)