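; Moving platform actor that travels along the spline of a BP_PlatformSpline actor in the level.
; On BeginPlay it finds that spline actor with GetActorOfClass, stores it in ChooseSpline and starts the Move timeline at a play rate set by Speed.
; Each timeline update maps the Move track value to a distance along the spline and places the platform at that world location.
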(event `self.ReceiveBeginPlay`
  (bind _returnvalue (`GameplayStatics.GetActorOfClass` "/Game/My_Work/BluePrint/BP_PlatformSpline.BP_PlatformSpline_C"))
  (set `self.Choose Spline` _returnvalue)
  (`self.Moving Platform`))

(event `Moving Platform`
  (`TimelineComponent.SetPlayRate` (`self.Move`) (`self.Speed`))
  (bind (_direction _move) (`Timeline|Move`)
    (:`Update`
      (`self.K2_SetActorTransform` (`KismetMathLibrary.MakeTransform` (`SplineComponent.GetLocationAtDistanceAlongSpline` (`/Game/My_Work/BluePrint/BP_PlatformSpline.Spline` (`self.Choose Spline`)) (`KismetMathLibrary.Lerp` 0.0 (`SplineComponent.GetSplineLength` (`/Game/My_Work/BluePrint/BP_PlatformSpline.Spline` (`self.Choose Spline`))) _move) "World"))))))

(fn `UserConstructionScript`)