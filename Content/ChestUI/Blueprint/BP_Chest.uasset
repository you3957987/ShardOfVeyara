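; BP_Chest is a chest actor that opens a chest and inventory UI for the BP_Farmer player.
; It passes its slots to its chest component and caches the player at BeginPlay.
; One OpenChestUI event initializes both HUD widgets with chest and player components, then toggles the player's open state.
; A second OpenChestUI event instead creates a WBP_ChestAndInventory widget, enabling Game-and-UI input and the mouse cursor.
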(event `self.ReceiveBeginPlay`
  (set `/Game/ChestUI/Blueprint/BPAC_ChestComponent.Chest Slots` (`self.ChestSlots`) (`self.BPAC_ChestComponent`))
  (bind _asbp_farmer (cast `/Game/HYH/Blueprints/BP_Farmer` (`GameplayStatics.GetPlayerPawn` 0)))
  (set `self.PlayerRef` _asbp_farmer))

(event `Toggle Chest`
  (bind _playerref (`self.PlayerRef`))
  (bind _returnvalue (not (`/Game/HYH/Blueprints/BP_Farmer.isChestOpened?` (`self.PlayerRef`))))
  (`/Game/ChestUI/Blueprint/WBP_ChestAndInventory.Toogle Chest` (`/Game/HYH/Blueprints/BP_Farmer.Chest HUD Ref` _playerref) _returnvalue)
  (set `/Game/HYH/Blueprints/BP_Farmer.isChestOpened?` _returnvalue _playerref))

(event `self.Open_Chest_UI`
  (bind _playerref (`self.PlayerRef`))
  (bind _playerref_2 (`self.PlayerRef`))
  (bind _chest_hud_ref (`/Game/HYH/Blueprints/BP_Farmer.Chest HUD Ref` (`self.PlayerRef`)))
  (`AGSDCharacter.SetCanOpenChest` _playerref_2 false)
  (set `/Game/HYH/Blueprints/BP_Farmer.CurrentChest` null _playerref_2)
  (`/Game/ChestUI/Blueprint/WBP_ChestUI.Initialize Chest` (`/Game/ChestUI/Blueprint/WBP_ChestAndInventory.WBP_ChestUI` _chest_hud_ref) self (`self.BPAC_ChestComponent`) 5)
  (`/Game/Inventory/Blueprint/UI/WBP_InventoryUI.Initialize Inventory` (`/Game/ChestUI/Blueprint/WBP_ChestAndInventory.WBP_InventoryUI` _chest_hud_ref) _playerref (`/Game/HYH/Blueprints/BP_Farmer.BPAC_InventoryComponent` _playerref) 5)
  (`self.Toggle Chest`))

(event `OpenChestUI`
  (bind _returnvalue (`GameplayStatics.GetPlayerController` 0))
  (`self.OpenChest`)
  (`WidgetBlueprintLibrary.SetInputMode_GameAndUIEx` _returnvalue null)
  (set `PlayerController.bShowMouseCursor` true _returnvalue))

(fn `OpenChest`
  (bind _returnvalue (`|CreateWidget` "/Game/ChestUI/Blueprint/WBP_ChestAndInventory.WBP_ChestAndInventory_C"))
  (`UserWidget.AddToViewport` _returnvalue 0))

(fn `UserConstructionScript`)