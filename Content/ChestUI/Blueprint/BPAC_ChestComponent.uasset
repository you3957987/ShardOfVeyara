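; Actor component that holds a chest's item slots for the chest UI, with functions to add, move and clear items.
; AddItem finds the first slot flagged empty, builds item data from DT_InventoryItemData plus the amount, and calls OnItemAdded.
; Drag-and-drop updates rewrite the matching slot and refresh its widget, while clearing flags a slot empty and calls OnItemRemoved.
; InitializeSlot builds the indexed slot array but is disconnected from BeginPlay.
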(event `self.ReceiveBeginPlay`)

(fn `Add Item`
  (params (`Item ID` :type String) (Amount :type Integer))
  (returns (`Success?` :type Boolean))
  (bind (_empty_slot_available _index) (`self.Check For Empty Slots`))
  (if _empty_slot_available
    (bind _returnvalue (`|GetDataTableRow` "/Game/Inventory/Blueprint/Item/DT_InventoryItemData.DT_InventoryItemData" (`KismetStringLibrary.Conv_StringToName` (`local.Item ID`)))
      (:`then`
        (bind _structout (setmembers `/Game/Inventory/Blueprint/Item/Struct_ItemData` :`StructRef` _returnvalue :`Current Quantity` (+ (`.CurrentQuantity_14_8774301F4880F214D37429B27F09B3CB` (break `/Game/Inventory/Blueprint/Item/Struct_ItemData` _returnvalue)) (`local.Amount`))))
        (bind _structout_2 (setmembers `/Game/ChestUI/Blueprint/Struct_ChestSlotData` :`StructRef` (`|GetArrayItem` (`self.Chest Slots`) _index) :`isEmpty` true :`ItemData` _structout))
        (`self.OnItemAdded` _structout_2)
        (return false)))))

(fn `Check For Empty Slots`
  (returns (`Empty Slot Available` :type Boolean) (Index :type Integer))
  (for (_array_element _array_index) (`self.Chest Slots`)
    (if (`.isEmpty_2_2DBD0A4B4A733755660DA8AC482E4686` (break `/Game/ChestUI/Blueprint/Struct_ChestSlotData` _array_element))
      (`|ExecutionSequence`
        (:`then_0`
          (break))
        (:`then_1`
          (return true _array_index)))))
  (return false -1))

(fn `ClearChestSlot`
  (params (`Slot Data to Clear` :type "/Game/ChestUI/Blueprint/Struct_ChestSlotData Structure"))
  (bind _structout (setmembers `/Game/ChestUI/Blueprint/Struct_ChestSlotData` :`StructRef` (`|GetArrayItem` (`self.Chest Slots`) (`.SlotIndex_7_B90779A34435FEC1F62A16805BB8506D` (break `/Game/ChestUI/Blueprint/Struct_ChestSlotData` `Slot Data to Clear`))) :`isEmpty` true :`ItemData` (struct :`ItemCategory` "NewEnumerator0")))
  (`self.OnItemRemoved` _structout))

(fn `Initialize Slot`
  (for _index (range (`self.Num of Chest Slots`))
    (`KismetArrayLibrary.Array_Add` (`self.Chest Slots`) (make `/Game/ChestUI/Blueprint/Struct_ChestSlotData` false (struct :`ItemCategory` "NewEnumerator0") _index))))

(fn `Update Slot (Drag and Drop)`
  (params (`Slot To Update` :type "/Game/ChestUI/Blueprint/WBP_ChestSlot Object Reference") (`New Slot Data` :type "/Game/ChestUI/Blueprint/Struct_ChestSlotData Structure") (`Chest Slot To Update` :type "/Game/ChestUI/Blueprint/WBP_ChestSlot Object Reference"))
  (bind (_isempty _itemdata) (break `/Game/ChestUI/Blueprint/Struct_ChestSlotData` `New Slot Data`))
  (bind _chest_slots (`self.Chest Slots`))
  (bind _returnvalue (`KismetArrayLibrary.Array_Find` _chest_slots (`/Game/ChestUI/Blueprint/WBP_ChestSlot.Chest Slot Data` `Slot To Update`)))
  (`|ExecutionSequence`
    (:`then_0`
      (if (!= _returnvalue -1)
        (setmembers `/Game/ChestUI/Blueprint/Struct_ChestSlotData` :`StructRef` (`|GetArrayItem` _chest_slots _returnvalue) :`isEmpty` _isempty :`ItemData` _itemdata))
      (bind _structout (setmembers `/Game/ChestUI/Blueprint/Struct_ChestSlotData` :`StructRef` (`/Game/ChestUI/Blueprint/WBP_ChestSlot.Chest Slot Data` `Slot To Update`) :`isEmpty` _isempty :`ItemData` _itemdata))
      (`/Game/ChestUI/Blueprint/WBP_ChestSlot.Init/Update Slot` (`local.Slot To Update`) _structout))))