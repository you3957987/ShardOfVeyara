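; BP_Harvest is a harvestable actor that gives an item to the farmer player who interacts with it.
; HarvestInteract casts the player to BP_Farmer and adds its ItemID and Amount to the farmer's inventory component.
; Only when the add succeeds does it show an item notification on the player HUD and destroy itself.
; BeginPlay, overlap, Tick and the construction script are empty.
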(event `self.HarvestInteract`
  (params (player :type "AGSDCharacter Object Reference"))
  (bind _asbp_farmer (cast `/Game/HYH/Blueprints/BP_Farmer` player))
  (bind _success_ (`/Game/Inventory/Blueprint/Inventory/BPAC_InventoryComponent.Add Item` (`/Game/HYH/Blueprints/BP_Farmer.BPAC_InventoryComponent` _asbp_farmer) (`self.ItemID`) (`self.Amount`)))
  (if _success_
    (`/Game/Inventory/Blueprint/UI/WBP_PlayerHUD.Add Item Notification` (`/Game/HYH/Blueprints/BP_Farmer.Player HUD Ref` _asbp_farmer) (`self.Item Data Struct`) (`self.Amount`))
    (`self.K2_DestroyActor`)))

(fn `UserConstructionScript`)