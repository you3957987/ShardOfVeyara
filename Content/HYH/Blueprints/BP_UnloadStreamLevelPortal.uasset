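; Portal actor that hides a streamed sublevel and teleports the player when the player pawn overlaps its box.
; On overlap it stores its teleport tag in BP_GameInstance, plays audio and sets ShouldBeVisible to false on the named streaming level, without calling an unload.
; It then moves the pawn to the location and rotation of the PlayerStart that the game mode finds by that tag.
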(event `self.Box.OnComponentBeginOverlap`
  (params (OverlappedComponent :type "PrimitiveComponent Object Reference") (OtherActor :type "Actor Object Reference") (OtherComp :type "PrimitiveComponent Object Reference") (OtherBodyIndex :type Integer) (bFromSweep :type Boolean) (SweepResult :type "HitResult Structure (by ref)"))
  (if (== OtherActor (`GameplayStatics.GetPlayerPawn` 0))
    (bind _asbp_game_instance (cast `/Game/LevelDesign/BluePrint/BP_GameInstance` (`GameplayStatics.GetGameInstance`)))
    (bind _output_get (set `SOVGameInstance.TeleportationTag` (`self.Tele Tag`) _asbp_game_instance))
    (`AudioComponent.Play` (`self.Audio`) 0.0)
    (set `LevelStreaming.bShouldBeVisible` false (`GameplayStatics.GetStreamingLevel` (`self.UnloadLevelName`)))
    (bind (_returnvalue_location _returnvalue_rotation) (`KismetMathLibrary.BreakTransform` (`self.GetTransform` (`GameModeBase.K2_FindPlayerStart` (`GameplayStatics.GetGameMode`) (`GameplayStatics.GetPlayerController` 0) (`KismetStringLibrary.Conv_NameToString` _output_get)))))
    (`self.K2_SetActorLocationAndRotation` (`GameplayStatics.GetPlayerPawn` 0) _returnvalue_location _returnvalue_rotation false false)))

(fn `UserConstructionScript`)