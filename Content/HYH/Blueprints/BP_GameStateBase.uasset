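; BP_GameStateBase is a game state that holds the current day and time and carries them across its lifetime through BP_GameInstance.
; On BeginPlay it copies CurrentDay and CurrentTime from the game instance.
; On EndPlay it writes both values back, so the game instance serves as the persistent store.
; It does not advance time itself, as Tick is empty.
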(event `self.ReceiveBeginPlay`
  (bind _asbp_game_instance (cast `/Game/LevelDesign/BluePrint/BP_GameInstance` (`GameplayStatics.GetGameInstance`)))
  (set `self.CurrentDay` (`/Game/LevelDesign/BluePrint/BP_GameInstance.CurrentDay` _asbp_game_instance))
  (set `self.CurrentTime` (`/Game/LevelDesign/BluePrint/BP_GameInstance.CurrentTime` _asbp_game_instance)))

(event `self.ReceiveEndPlay`
  (params (EndPlayReason :type "EEndPlayReason Enum" :default "Destroyed"))
  (bind _asbp_game_instance (cast `/Game/LevelDesign/BluePrint/BP_GameInstance` (`GameplayStatics.GetGameInstance`)))
  (set `/Game/LevelDesign/BluePrint/BP_GameInstance.CurrentDay` (`self.CurrentDay`) _asbp_game_instance)
  (set `/Game/LevelDesign/BluePrint/BP_GameInstance.CurrentTime` (`self.CurrentTime`) _asbp_game_instance))

(fn `UserConstructionScript`)