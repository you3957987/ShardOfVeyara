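; BP_WeaponBase is a weapon Blueprint that runs a normal and a strong attack on the player passed to it.
; Each attack sets the player's Mining and SkillMotion flags, writes its damage to the player and plays its montage on the player's mesh.
; A per-attack timer clears SkillMotion, while Mining clears only when the montage completes, with no handling for interruption.
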(event `Attack`
  (params (Player :type "/Game/HYH/Blueprints/BP_Farmer Object Reference"))
  (set `AGSDCharacter.Mining` true Player)
  (set `AGSDCharacter.SkillMotion` true Player)
  (bind _returnvalue (`KismetSystemLibrary.K2_SetTimerDelegate` (delegate `SetAttackSkillMotion`) (`self.AttackTime`)))
  (set `self.SetSkillMotionTimer` _returnvalue)
  (set `/Game/HYH/Blueprints/BP_Farmer.Damage` (`self.AttackDamage`) Player)
  (`|PlayMontage` (`Character.Mesh` Player) (`self.AttackMontage`)
    (:`OnCompleted`
      (set `AGSDCharacter.Mining` false Player))))

(event `SetAttackSkillMotion`
  (set `AGSDCharacter.SkillMotion` false (stale `Attack` Player)))

(event `StrongAttack`
  (params (Player :type "/Game/HYH/Blueprints/BP_Farmer Object Reference"))
  (set `AGSDCharacter.Mining` true Player)
  (set `AGSDCharacter.SkillMotion` true Player)
  (bind _returnvalue (`KismetSystemLibrary.K2_SetTimerDelegate` (delegate `SetStrongAttackSkillMontion`) (`self.StrongAttackTime`)))
  (set `self.SetSkillMotionTimer` _returnvalue)
  (set `/Game/HYH/Blueprints/BP_Farmer.Damage` (`self.StrongAttackDamage`) Player)
  (`|PlayMontage` (`Character.Mesh` Player) (`self.StrongAttackMontage`)
    (:`OnCompleted`
      (set `AGSDCharacter.Mining` false Player))))

(event `SetStrongAttackSkillMontion`
  (set `AGSDCharacter.SkillMotion` false (stale `StrongAttack` Player)))

(fn `UserConstructionScript`
  (`parent.UserConstructionScript`))