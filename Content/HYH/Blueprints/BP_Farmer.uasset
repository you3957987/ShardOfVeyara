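; BP_Farmer is the player farmer character, handling the HUD, inventory and chest toggles, pause menu and held-item combat.
; Tick watches the hand slot's item ID and, for tools, respawns the held actor on a mesh socket.
; Attack events forward to the held BP_WeaponBase and toggle its hit sensor collision.
; SubSeedAmount decrements the held seed stack; saving records player location, but restoring it on load is unwired.
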(event `EnhancedInput|/Game/ChestUI/Input/IA_OpenChest`
  (params (ActionValue :type Boolean) (ElapsedSeconds :type "Float (double-precision)") (TriggeredSeconds :type "Float (double-precision)") (InputAction :type "InputAction Object Reference" :default "/Game/ChestUI/Input/IA_OpenChest.IA_OpenChest"))
  (bind _returnvalue (not (`self.isInventoryOpened?`)))
  (:`Started`
    (if (not (`self.Mining`))
      (`/Game/Inventory/Blueprint/UI/WBP_PlayerHUD.Toogle Inventory` (`self.Player HUD Ref`) _returnvalue :!label _label)
      (set `self.isInventoryOpened?` _returnvalue))))

(event `EnhancedInput|/Game/Inventory/Blueprint/Input/IA_OpenInventory`
  (params (ActionValue :type Boolean) (ElapsedSeconds :type "Float (double-precision)") (TriggeredSeconds :type "Float (double-precision)") (InputAction :type "InputAction Object Reference" :default "/Game/Inventory/Blueprint/Input/IA_OpenInventory.IA_OpenInventory"))
  (:`Started`
    (if (`self.Mining`)
      _
      (elif (`self.bCanOpenChest`)
        (goto _label)))))

(event `self.ReceiveBeginPlay`
  (`|ExecutionSequence`
    (:`then_0`
      (bind _returnvalue (`|CreateWidget` "/Game/Inventory/Blueprint/UI/WBP_PlayerHUD.WBP_PlayerHUD_C"))
      (bind _output_get (set `self.Player HUD Ref` _returnvalue))
      (`UserWidget.AddToViewport` _output_get 0))))

(event `self.ReceiveTick`
  (params (DeltaSeconds :type "Float (single-precision)"))
  (bind _handslot (`self.HandSlot`)
    (:`then`
      (bind _itemid (break `/Game/Inventory/Blueprint/Item/Struct_ItemData` (`.ItemData_5_B5994FE14A98159059BA1CA99CAC5E74` (break `/Game/Inventory/Blueprint/Inventory/Struct_InventorySlotData` (`/Game/Inventory/Blueprint/UI/Hotbar/WBP_HotbarSlot.Hotbar Item` _handslot)))))
      (if (`KismetStringLibrary.NotEqual_StrStr` _itemid (`self.PrevItemID`))
        (set `self.PrevItemID` _itemid)
        (bind _holdingactor (`self.HoldingActor`)
          (:`then`
            (`self.K2_DestroyActor` _holdingactor))
          (:`else`
            _))
        (if (`|EnumEquality` (`self.HoldingState`) "EHS_Tool")
          (bind _asbp_pick_up_item_base (castclass `/Game/HYH/Blueprints/BP_PickUpItemBase` (`.ItemBPClass_20_1698E4734C0F220DEF27D0BB37C5CF2B` (break `/Game/Inventory/Blueprint/Item/Struct_ItemData` (`.ItemData_5_B5994FE14A98159059BA1CA99CAC5E74` (break `/Game/Inventory/Blueprint/Inventory/Struct_InventorySlotData` (`/Game/Inventory/Blueprint/UI/Hotbar/WBP_HotbarSlot.Hotbar Item` (`self.HandSlot`))))))))
          (bind _returnvalue (`|SpawnActorFromClass` _asbp_pick_up_item_base (`self.GetTransform`) "Undefined" "MultiplyWithRoot" null true null))
          (set `self.HoldingActor` _returnvalue)
          (bind _holdingactor_2 (`self.HoldingActor`)
            (:`then`
              (`self.K2_AttachToComponent` _holdingactor_2 (`self.Mesh`) (`KismetMathLibrary.SelectName` "SenseSocket" "weaponSocket" (`KismetStringLibrary.EqualEqual_StrStr` (`self.PrevItemID`) "Sence")) "SnapToTarget" "SnapToTarget" "KeepWorld" true))
            (:`else`)))))
    (:`else`)))

(event `self.Attack`
  (bind _asbp_weapon_base (cast `/Game/HYH/Blueprints/Weapons/BP_WeaponBase` (`self.HoldingActor`)))
  (`/Game/HYH/Blueprints/Weapons/BP_WeaponBase.Attack` _asbp_weapon_base self))

(event `Key|K`
  (params (Key :type "Key Structure"))
  (:`Pressed`
    (bind _chest_hud_ref (`self.Chest HUD Ref`)
      (:`then`
        (`/Game/ChestUI/Blueprint/WBP_ChestAndInventory.Toogle Chest` _chest_hud_ref false)
        (`Widget.RemoveFromParent` (`self.Chest HUD Ref`))
        (set `self.Chest HUD Ref` null)
        (set `self.OpenedChest` null)
        (set `self.bCanOpenChest` true))
      (:`else`))))

(event `self.StrongAttack`
  (bind _asbp_weapon_base (cast `/Game/HYH/Blueprints/Weapons/BP_WeaponBase` (`self.HoldingActor`)))
  (`/Game/HYH/Blueprints/Weapons/BP_WeaponBase.StrongAttack` _asbp_weapon_base self))

(event `EnhancedInput|/Game/HYH/Input/IA_Attack`
  (params (ActionValue :type Boolean) (ElapsedSeconds :type "Float (double-precision)") (TriggeredSeconds :type "Float (double-precision)") (InputAction :type "InputAction Object Reference" :default "/Game/HYH/Input/IA_Attack.IA_Attack"))
  (:`Triggered`
    (if (`|EnumEquality` (`self.HoldingState`) "EHS_Tool")
      (`self.HandleAttackInput` "Attack")
      (`KismetSystemLibrary.PrintString` "Hello"))))

(event `self.WeaponAttack`
  (`self.Attacking`
    (:`then`
      (set `self.Attacking` false)
      (bind _holdingactor (`self.HoldingActor`)
        (:`then`
          (bind _asbp_weapon_base (cast `/Game/HYH/Blueprints/Weapons/BP_WeaponBase` _holdingactor))
          (`PrimitiveComponent.SetCollisionEnabled` (`/Game/HYH/Blueprints/Weapons/BP_WeaponBase.AttackSensor` _asbp_weapon_base) "NoCollision"))
        (:`else`)))
    (:`else`
      (set `self.Attacking` true)
      (bind _holdingactor_2 (`self.HoldingActor`)
        (:`then`
          (bind _asbp_weapon_base_2 (cast `/Game/HYH/Blueprints/Weapons/BP_WeaponBase` _holdingactor_2))
          (`PrimitiveComponent.SetCollisionEnabled` (`/Game/HYH/Blueprints/Weapons/BP_WeaponBase.AttackSensor` _asbp_weapon_base_2) "QueryOnly"))
        (:`else`)))))

(event `EnhancedInput|/Game/MainMenuUI/Input/IA_Pause`
  (params (ActionValue :type Boolean) (ElapsedSeconds :type "Float (double-precision)") (TriggeredSeconds :type "Float (double-precision)") (InputAction :type "InputAction Object Reference" :default "/Game/MainMenuUI/Input/IA_Pause.IA_Pause"))
  (bind _returnvalue (`GameplayStatics.GetPlayerController` 0))
  (:`Started`
    (bind _returnvalue_2 (`|CreateWidget` "/Game/MainMenuUI/Blueprint/WBP_PauseMenu.WBP_PauseMenu_C"))
    (`UserWidget.AddToViewport` _returnvalue_2 0)
    (set `PlayerController.bShowMouseCursor` true _returnvalue)
    (`WidgetBlueprintLibrary.SetInputMode_UIOnlyEx` _returnvalue null)
    (`GameplayStatics.SetGamePaused` true)))

(event `/Game/HYH/Blueprints/BI_SaveGame.OnGameSaved`
  (params (savedSuccessfully :type Boolean)))

(event `/Game/HYH/Blueprints/BI_SaveGame.OnGameLoaded`
  (params (`HasSaveGame?` :type Boolean) (LoadedGameData :type "/Game/HYH/Blueprints/Struct_SaveGameData Structure"))
  (if `HasSaveGame?`
    _))

(fn `OnPreSave`
  (params (InitialSaveGameObject :type "/Game/HYH/Blueprints/Struct_SaveGameData Structure"))
  (returns (OutputSaveGameStruct :type "/Game/HYH/Blueprints/Struct_SaveGameData Structure") (Implemented :type Boolean))
  (bind _structout (setmembers `/Game/HYH/Blueprints/Struct_SaveGameData` :`StructRef` InitialSaveGameObject :`LastPlayerLocation` (`self.K2_GetActorLocation`)))
  (return _structout true))

(fn `SubSeedAmount`
  (returns (ReturnValue :type String))
  (locals (ItemID :type String) (TempItemStruct :type "/Game/Inventory/Blueprint/Item/Struct_ItemData Structure"))
  (bind _handslot (`self.HandSlot`))
  (bind (_isempty _item_data _slot_index) (`/Game/Inventory/Blueprint/UI/Hotbar/WBP_HotbarSlot.Get Hotbar Item` _handslot))
  (bind (_itemid _itemcategory _itemname _itemdescription _maxquantity _currentquantity _itemicon _itembpclass _isequipmentequipped_) (break `/Game/Inventory/Blueprint/Item/Struct_ItemData` _item_data))
  (`parent.SubSeedAmount`)
  (set `local.ItemID` _itemid)
  (bind _result (`/Engine/EditorBlueprintResources/StandardMacros.DecrementInt` _currentquantity)
    (:`  `
      (bind _output_get (set `local.TempItemStruct` (make `/Game/Inventory/Blueprint/Item/Struct_ItemData` _itemid _itemcategory _itemname _itemdescription _maxquantity _result _itemicon _itembpclass _isequipmentequipped_)))
      (bind _returnvalue (<= _result 0))
      (`/Game/Inventory/Blueprint/UI/Hotbar/WBP_HotbarSlot.Set Hotbar Item` _handslot _output_get _returnvalue)
      (if _returnvalue
        (bind _result_2 (`/Engine/EditorBlueprintResources/StandardMacros.IncrementInt` _slot_index)
          (:`  `
            (`/Game/Inventory/Blueprint/Inventory/BPAC_InventoryComponent.OnHotbarSelected` (`self.BPAC_InventoryComponent`) _result_2))))
      (return (`local.ItemID`)))))

(fn `UserConstructionScript`)