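; BP_TutorialWidget is a trigger-box actor that shows a tutorial text widget when the BP_Farmer enters it.
; The WBP_TutorialWidget is removed after a short timer or when the farmer leaves the box.
; On exit, if NewVar is valid, it unhides that actor, sets its SetCollisionEnable and destroys itself, allowing chained tutorial steps.
; Both overlap events are gated by this trigger's own SetCollisionEnable.
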(event `self.TriggerBox.OnComponentBeginOverlap`
  (params (OverlappedComponent :type "PrimitiveComponent Object Reference") (OtherActor :type "Actor Object Reference") (OtherComp :type "PrimitiveComponent Object Reference") (OtherBodyIndex :type Integer) (bFromSweep :type Boolean) (SweepResult :type "HitResult Structure (by ref)"))
  (`self.SetCollisionEnable`
    (:`then`
      (cast `/Game/HYH/Blueprints/BP_Farmer` OtherActor)
      (bind _returnvalue (`|CreateWidget` "/Game/HYH/Blueprints/Widgets/WBP_TutorialWidget.WBP_TutorialWidget_C" (`GameplayStatics.GetPlayerController` 0) (`self.Text`)))
      (bind _output_get (set `self.ref` _returnvalue))
      (`UserWidget.AddToViewport` _returnvalue 0)
      (`UserWidget.AddToViewport` _output_get 0)
      (`KismetSystemLibrary.K2_SetTimerDelegate` (delegate `커스텀이벤트`) 2.0))
    (:`else`)))

(event `커스텀이벤트`
  (bind _ref (`self.ref` :!label _label)
    (:`then`
      (`Widget.RemoveFromParent` _ref))
    (:`else`)))

(event `self.TriggerBox.OnComponentEndOverlap`
  (params (OverlappedComponent :type "PrimitiveComponent Object Reference") (OtherActor :type "Actor Object Reference") (OtherComp :type "PrimitiveComponent Object Reference") (OtherBodyIndex :type Integer))
  (`self.SetCollisionEnable`
    (:`then`
      (cast `/Game/HYH/Blueprints/BP_Farmer` OtherActor)
      (`|ExecutionSequence`
        (:`then_0`
          (goto _label))
        (:`then_1`
          (bind _newvar (`self.NewVar`)
            (:`then`
              (`self.SetActorHiddenInGame` _newvar false)
              (set `/Game/HYH/Blueprints/BP_TutorialWidget.SetCollisionEnable` true _newvar)
              (`self.K2_DestroyActor`))
            (:`else`)))))
    (:`else`)))

(fn `UserConstructionScript`)