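; BP_Tribute is an interaction actor that drives fire effects on a tribute object.
; PlayFireNiagara plays a timeline that feeds scaled spawn rate, sphere radius and velocity values into the NSFire Niagara component.
; PlayFireExplosionNiagara spawns a self-destroying explosion system attached to NSFire.
; BeginPlay sets a looping timer with no visible bound event, and nothing in this graph calls either fire event.
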(event `self.ReceiveBeginPlay`
  (`KismetSystemLibrary.K2_SetTimerDelegate` :`Time` 3.0 :`bLooping` true))

(event `self.PlayFireNiagara`
  (bind _ns_fire (`self.NS_Fire`))
  (bind (_direction _spawnrate _sphereradius _velocityspeedscale) (`Timeline|타임라인` :!via `PlayFromStart`)
    (:`Update`
      (`|ExecutionSequence`
        (:`then_0`
          (`NiagaraComponent.SetVariableFloat` _ns_fire "User.SpawnRate" (* _spawnrate 250.0)))
        (:`then_1`
          (`NiagaraComponent.SetVariableFloat` _ns_fire "User.SphereRadius" (* _sphereradius 20.0)))
        (:`then_2`
          (`NiagaraComponent.SetVariableFloat` _ns_fire "User.VelocitySpeedScale" (* _velocityspeedscale 1.0)))))))

(event `self.PlayFireExplosionNiagara`
  (`NiagaraFunctionLibrary.SpawnSystemAttached` "/Game/HYH/Niagaras/NS_FireExplosion.NS_FireExplosion" (`self.NS_Fire`) "None" (0.0 0.0 0.0) (struct) "KeepRelativeOffset" true))

(fn `UserConstructionScript`)