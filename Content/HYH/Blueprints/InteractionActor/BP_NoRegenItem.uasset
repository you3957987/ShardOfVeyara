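; BP_NoRegenItem is an interactable pickup item that does not respawn once it has been collected.
; On pickup it calls AddItemFunction with its item data, then adds a key built from level name plus object name to the GameInstance's NoRegenItem array.
; On BeginPlay it looks up that key in the array and destroys itself if found, so collected items stay gone when the level loads again.
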(event `self.ReceiveBeginPlay`
  (bind _asbp_game_instance (cast `/Game/LevelDesign/BluePrint/BP_GameInstance` (`GameplayStatics.GetGameInstance`)))
  (bind _returnvalue (`GameplayStatics.GetCurrentLevelName` true))
  (if (!= (`KismetArrayLibrary.Array_Find` (`/Game/LevelDesign/BluePrint/BP_GameInstance.NoRegenItem` _asbp_game_instance) (`KismetStringLibrary.Concat_StrStr` _returnvalue (`KismetSystemLibrary.GetObjectName` self))) -1)
    (`self.K2_DestroyActor`)))

(event `self.PickUpInteract`
  (params (player :type "AGSDCharacter Object Reference"))
  (`/Game/HYH/Blueprints/BPFL.AddItemFunction` player (`self.ItemID`) (`self.Amount`) (`self.Item Data Struct`) self)
  (bind _asbp_game_instance (cast `/Game/LevelDesign/BluePrint/BP_GameInstance` (`GameplayStatics.GetGameInstance`)))
  (bind _returnvalue (`GameplayStatics.GetCurrentLevelName` true))
  (`KismetArrayLibrary.Array_AddUnique` (`/Game/LevelDesign/BluePrint/BP_GameInstance.NoRegenItem` _asbp_game_instance) (`KismetStringLibrary.Concat_StrStr` _returnvalue (`KismetSystemLibrary.GetObjectName` self))))

(fn `UserConstructionScript`
  (`parent.UserConstructionScript`))