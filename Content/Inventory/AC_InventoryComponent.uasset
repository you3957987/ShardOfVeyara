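; Inventory component whose logic is currently disconnected: BeginPlay is empty and none of the other chains run.
; The unwired chains create an 18-slot inventory widget and toggle it with cursor and input mode changes.
; A pickup chain sphere-traces at the owner's feet for a BP_Item, stacks it up to 64 or fills an empty slot, then refreshes the widget and destroys the item.
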(event `self.ReceiveBeginPlay`)

(event `Key|I`
  (params (Key :type "Key Structure")))

(event `Key|E`
  (params (Key :type "Key Structure")))