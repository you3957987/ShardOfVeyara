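; Inventory component that holds an actor's item slots and, on the farmer, drives hotbar selection by scroll or number keys.
; Adds items from a data table by filling partial stacks then empty slots, and handles removal, drag-and-drop and dropping items as ground-traced pickups.
; Changes call notify functions for listeners.
; The farmer carries slots and selection between levels through the GameInstance, except slots leaving Tutorial_Village; save-game hooks are unwired.
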(event `EnhancedInput|/Game/Inventory/Blueprint/Input/IA_SelectHotbarScroll`
  (params (ActionValue :type "Float (double-precision)") (ElapsedSeconds :type "Float (double-precision)") (TriggeredSeconds :type "Float (double-precision)") (InputAction :type "InputAction Object Reference" :default "/Game/Inventory/Blueprint/Input/IA_SelectHotbarScroll.IA_SelectHotbarScroll"))
  (:`Triggered`
    (bind _asbp_farmer (cast `/Game/HYH/Blueprints/BP_Farmer` (`self.GetOwner`)))
    (if (`AGSDCharacter.Mining` _asbp_farmer)
      _
      (elif (== ActionValue -1.0)
        (`self.SelectHotbar` (+ (`self.CurrentSelectedHotbar`) 1))
        (elif (== ActionValue 1.0)
          (`self.SelectHotbar` (+ (`self.CurrentSelectedHotbar`) -1)))))))

(event `EnhancedInput|/Game/Inventory/Blueprint/Input/IA_SelectHotbar`
  (params (ActionValue :type Boolean) (ElapsedSeconds :type "Float (double-precision)") (TriggeredSeconds :type "Float (double-precision)") (InputAction :type "InputAction Object Reference" :default "/Game/Inventory/Blueprint/Input/IA_SelectHotbar.IA_SelectHotbar"))
  (:`Ongoing`
    (bind _asbp_farmer (cast `/Game/HYH/Blueprints/BP_Farmer` (`self.GetOwner`)))
    (if (not (`AGSDCharacter.Mining` _asbp_farmer))
      (for _array_element (`EnhancedInputSubsystemInterface.QueryKeysMappedToAction` (pcsubsystem `EnhancedInputLocalPlayerSubsystem` (`GameplayStatics.GetPlayerController` 0)) "/Game/Inventory/Blueprint/Input/IA_SelectHotbar.IA_SelectHotbar")
        (if (`PlayerController.IsInputKeyDown` (`GameplayStatics.GetPlayerController` 0) _array_element)
          (`self.SelectHotbar` (`KismetStringLibrary.Conv_StringToInt` (`KismetTextLibrary.Conv_TextToString` (`KismetInputLibrary.Key_GetDisplayName` _array_element)))))))))

(event `self.ReceiveEndPlay`
  (params (EndPlayReason :type "EEndPlayReason Enum" :default "Destroyed"))
  (cast `/Game/HYH/Blueprints/BP_Farmer` (`self.GetOwner`))
  (bind _asbp_game_instance (cast `/Game/LevelDesign/BluePrint/BP_GameInstance` (`GameplayStatics.GetGameInstance`)))
  (set `/Game/LevelDesign/BluePrint/BP_GameInstance.CurrentSelectedHotbar` (`self.CurrentSelectedHotbar`) _asbp_game_instance)
  (bind _returnvalue (`GameplayStatics.GetCurrentLevelName` true))
  (if (not (`KismetStringLibrary.EqualEqual_StrStr` _returnvalue "Tutorial_Village"))
    (set `/Game/LevelDesign/BluePrint/BP_GameInstance.TempInventory` (`self.InventorySlots`) _asbp_game_instance)))

(event `self.ReceiveBeginPlay`
  (cast `/Game/HYH/Blueprints/BP_Farmer` (`self.GetOwner`)
    (:`then`
      (set `self.Num of Inventory Slots` 20)
      (bind _asbp_game_instance (cast `/Game/LevelDesign/BluePrint/BP_GameInstance` (`GameplayStatics.GetGameInstance`)))
      (bind _tempinventory (`/Game/LevelDesign/BluePrint/BP_GameInstance.TempInventory` _asbp_game_instance))
      (if (`KismetArrayLibrary.Array_IsEmpty` _tempinventory)
        ; 임시(savegame 구현 시 삭제)
        (`self.Initialize Slot`)
        (else
          (set `self.InventorySlots` _tempinventory)))
      (`KismetSystemLibrary.Delay` 0.1)
      (`self.SelectHotbar` (`/Game/LevelDesign/BluePrint/BP_GameInstance.CurrentSelectedHotbar` _asbp_game_instance)))
    (:`CastFailed`
      (`self.Initialize Slot`))))

(event `/Game/HYH/Blueprints/WorldSettings/BI_SaveGame.OnGameSaved`
  (params (savedSuccessfully :type Boolean)))

(event `/Game/HYH/Blueprints/WorldSettings/BI_SaveGame.OnGameLoaded`
  (params (`HasSaveGame?` :type Boolean) (LoadedGameData :type "/Game/HYH/Blueprints/Structs/Struct_SaveGameData Structure")))

(fn `Add Item`
  (params (`Item ID` :type String) (Amount :type Integer))
  (returns (`Success?` :type Boolean))
  (locals (`Item Data to Add` :type "/Game/Inventory/Blueprint/Item/Struct_ItemData Structure") (`Item Amount to Add` :type Integer) (`Item to Add` :type "/Game/Inventory/Blueprint/Item/Struct_ItemData Structure") (`Slot Add Amount` :type Integer :default 0))
  (bind _output_get (set `local.Item Amount to Add` Amount))
  (if (> _output_get 0)
    (bind _returnvalue (`|GetDataTableRow` "/Game/Inventory/Blueprint/Item/DT_InventoryItemData.DT_InventoryItemData" (`KismetStringLibrary.Conv_StringToName` `Item ID`))
      (:`then`
        (set `local.Item to Add` _returnvalue)
        (while (> (`local.Item Amount to Add`) 0)
          (bind (_slot_available _slot_index) (`self.Check For Existing Item Slot` (`local.Item to Add`)))
          (if (and (!= _slot_index -1) _slot_available)
            (bind _output (`|GetArrayItem` (`self.InventorySlots`) _slot_index))
            (bind (_isempty _itemdata) (break `/Game/Inventory/Blueprint/Inventory/Struct_InventorySlotData` _output))
            (bind (_itemid _itemcategory _itemname _itemdescription _maxquantity _currentquantity) (break `/Game/Inventory/Blueprint/Item/Struct_ItemData` _itemdata))
            (bind _returnvalue_2 (`KismetMathLibrary.Min` (- _maxquantity _currentquantity) (`local.Item Amount to Add`)))
            (if (> _returnvalue_2 0)
              (bind _output_get_2 (set `local.Slot Add Amount` _returnvalue_2))
              (bind _structout (setmembers `/Game/Inventory/Blueprint/Item/Struct_ItemData` :`StructRef` _itemdata :`Current Quantity` (+ _currentquantity _output_get_2)))
              (bind _structout_2 (setmembers `/Game/Inventory/Blueprint/Inventory/Struct_InventorySlotData` :`StructRef` _output :`ItemData` _structout))
              (`self.OnItemAdded` _structout_2)
              (bind _output_get_3 (set `local.Item Amount to Add` (- (`local.Item Amount to Add`) (`local.Slot Add Amount`))))
              (if (<= _output_get_3 0)
                (return true)))
            (else
              (bind (_empty_slot_available _index) (`self.Check For Empty Slost`))
              (if (and _empty_slot_available (!= _index -1))
                (bind _output_get_4 (set `local.Slot Add Amount` (`KismetMathLibrary.Min` (`.MaxQuantity_12_9FD6593140E036A33C5FEDAE0770BC8B` (break `/Game/Inventory/Blueprint/Item/Struct_ItemData` (`local.Item to Add`))) (`local.Item Amount to Add`))))
                (bind _structout_3 (setmembers `/Game/Inventory/Blueprint/Item/Struct_ItemData` :`StructRef` (`local.Item to Add`) :`Current Quantity` _output_get_4))
                (bind _structout_4 (setmembers `/Game/Inventory/Blueprint/Inventory/Struct_InventorySlotData` :`StructRef` (`|GetArrayItem` (`self.InventorySlots`) _index) :`isEmpty` false :`ItemData` _structout_3))
                (`self.OnItemAdded` _structout_4)
                (bind _output_get_5 (set `local.Item Amount to Add` (- (`local.Item Amount to Add`) (`local.Slot Add Amount`))))
                (if (<= _output_get_5 0)
                  (return true))
                (else
                  (`KismetSystemLibrary.PrintString` "Inventory Full")
                  (return false))))))))))

(fn `Check For Empty Slost`
  (returns (`Empty Slot Available` :type Boolean) (Index :type Integer))
  (for (_array_element _array_index) (`self.InventorySlots`)
    (if (`.isEmpty_2_6E75C8764B47955A3CECE3870E65F232` (break `/Game/Inventory/Blueprint/Inventory/Struct_InventorySlotData` _array_element))
      (`|ExecutionSequence`
        (:`then_0`
          (break))
        (:`then_1`
          (return true _array_index)))))
  (return false -1))

(fn `Check For Existing Item Slot`
  (params (`Item Data To Find` :type "/Game/Inventory/Blueprint/Item/Struct_ItemData Structure"))
  (returns (`Slot Available` :type Boolean) (`Slot Index` :type Integer))
  (for _array_element (`self.InventorySlots`)
    (bind (_isempty _itemdata _slotindex) (break `/Game/Inventory/Blueprint/Inventory/Struct_InventorySlotData` _array_element))
    (bind (_itemid _itemcategory _itemname _itemdescription _maxquantity _currentquantity) (break `/Game/Inventory/Blueprint/Item/Struct_ItemData` _itemdata))
    (if (and (`KismetStringLibrary.EqualEqual_StrStr` _itemid (`.ItemID_3_B1A8961D47BB4AF5F3223AAD8CCE5A5E` (break `/Game/Inventory/Blueprint/Item/Struct_ItemData` `Item Data To Find`))) (< _currentquantity _maxquantity))
      (`|ExecutionSequence`
        (:`then_0`
          (break))
        (:`then_1`
          (return true _slotindex)))))
  (return false -1))

(fn `ClearInventorySlot`
  (params (`Slot Data to Clear` :type "/Game/Inventory/Blueprint/Inventory/Struct_InventorySlotData Structure"))
  (bind _structout (setmembers `/Game/Inventory/Blueprint/Inventory/Struct_InventorySlotData` :`StructRef` (`|GetArrayItem` (`self.InventorySlots`) (`.SlotIndex_8_AA6E06B44888C3FA99CB0E8F3B0D2037` (break `/Game/Inventory/Blueprint/Inventory/Struct_InventorySlotData` `Slot Data to Clear`))) :`isEmpty` true :`ItemData` (struct :`ItemCategory` "EHS_None")))
  (`self.OnItemRemoved` _structout))

(fn `Drop Item`
  (params (`Inventory Slot` :type "/Game/Inventory/Blueprint/Inventory/Struct_InventorySlotData Structure") (`Dropping from Hotbar` :type Boolean))
  (bind (_isempty _itemdata _slotindex) (break `/Game/Inventory/Blueprint/Inventory/Struct_InventorySlotData` `Inventory Slot`))
  (bind (_itemid _itemcategory _itemname _itemdescription _maxquantity _currentquantity _itemicon _itembpclass) (break `/Game/Inventory/Blueprint/Item/Struct_ItemData` _itemdata))
  (bind (_itemid_2 _itemcategory_2 _itemname_2 _itemdescription_2 _maxquantity_2 _currentquantity_2 _itemicon_2 _itembpclass_2 _isequipmentequipped_) (break `/Game/Inventory/Blueprint/Item/Struct_ItemData` _itemdata))
  (bind _returnvalue (`Actor.K2_GetActorLocation` (`self.GetOwner`)))
  (`|ExecutionSequence`
    (:`then_0`
      (if _isequipmentequipped_
        (switch `string` _itemid_2)))
    (:`then_1`
      (if (not (`local.Dropping from Hotbar`))
        (bind _structout (setmembers `/Game/Inventory/Blueprint/Inventory/Struct_InventorySlotData` :`StructRef` (`|GetArrayItem` (`self.InventorySlots`) _slotindex) :`isEmpty` true :`ItemData` (struct :`ItemCategory` "EHS_None")))
        (`self.OnItemRemoved` _structout))
      (bind (_outhit _returnvalue_2) (`KismetSystemLibrary.LineTraceSingle` _returnvalue (+ _returnvalue (0.0 0.0 -2000.0)) "TraceTypeQuery1" false (`|MakeArray` (`self.GetOwner`))))
      (if _returnvalue_2
        (bind _returnvalue_3 (`|SpawnActorFromClass` _itembpclass (`KismetMathLibrary.MakeTransform` (+ (`.Location` (`GameplayStatics.BreakHitResult` _outhit)) (0.0 0.0 40.0))) "Undefined" "MultiplyWithRoot" null null))
        (bind _asbp_pick_up_item_base (cast `/Game/HYH/Blueprints/InteractionActor/BP_PickUpItemBase` _returnvalue_3))
        (set `/Game/HYH/Blueprints/InteractionActor/BP_PickUpItemBase.ItemID` _itemid _asbp_pick_up_item_base)
        (set `/Game/HYH/Blueprints/InteractionActor/BP_PickUpItemBase.Amount` _currentquantity _asbp_pick_up_item_base)
        (`/Game/HYH/Blueprints/InteractionActor/BP_PickUpItemBase.Initialize Item Data Structure` _asbp_pick_up_item_base)))))

(fn `Initialize Slot`
  (if (`KismetArrayLibrary.Array_IsEmpty` (`self.InventorySlots`))
    (for _index (range (`self.Num of Inventory Slots`))
      (`KismetArrayLibrary.Array_Add` (`self.InventorySlots`) (make `/Game/Inventory/Blueprint/Inventory/Struct_InventorySlotData` true (struct :`ItemCategory` "EHS_None") _index)))))

(fn `OnPreSave`
  (params (InitialSaveGameObject :type "/Game/HYH/Blueprints/Structs/Struct_SaveGameData Structure"))
  (returns (OutputSaveGameStruct :type "/Game/HYH/Blueprints/Structs/Struct_SaveGameData Structure") (Implemented :type Boolean)))

(fn `Remove Item`
  (params (`Item ID` :type String) (`Amount to Remove` :type Integer) (`Custom Slot Index` :type Integer :default -1))
  (locals (`Remaining To Remove` :type Integer) (`Updated Quantity` :type Integer))
  (bind _updated_quantity (`local.Updated Quantity`))
  (bind _output (`|GetArrayItem` (`self.InventorySlots`) `Custom Slot Index`))
  (bind _returnvalue (<= _updated_quantity 0))
  (bind (_isempty _itemdata) (break `/Game/Inventory/Blueprint/Inventory/Struct_InventorySlotData` _output))
  (set `local.Remaining To Remove` `Amount to Remove`)
  (if (!= `Custom Slot Index` -1)
    (set `local.Updated Quantity` (- (`.CurrentQuantity_14_8774301F4880F214D37429B27F09B3CB` (break `/Game/Inventory/Blueprint/Item/Struct_ItemData` _itemdata)) (`local.Remaining To Remove`)))
    (bind _structout (setmembers `/Game/Inventory/Blueprint/Item/Struct_ItemData` :`StructRef` _itemdata :`Current Quantity` _updated_quantity))
    (bind _structout_2 (setmembers `/Game/Inventory/Blueprint/Inventory/Struct_InventorySlotData` :`StructRef` _output :`isEmpty` (select `bool` _returnvalue :`true` true) :`ItemData` (select `bool` _returnvalue :`false` _structout)))
    (`self.OnItemRemoved` _structout_2)))

(fn `SelectHotbar`
  (params (`New Index` :type Integer))
  (if (!= `New Index` (`self.CurrentSelectedHotbar`))
    (bind _output_get (set `self.CurrentSelectedHotbar` (`KismetMathLibrary.SelectInt` 1 (`KismetMathLibrary.SelectInt` 10 `New Index` (== `New Index` 0)) (> `New Index` 10))))
    (`self.OnHotbarSelected` _output_get)))

(fn `Update Slot (Drag and Drop)`
  (params (`Slot To Update` :type "/Game/Inventory/Blueprint/UI/WBP_InventorySlot Object Reference") (`New Slot Data` :type "/Game/Inventory/Blueprint/Inventory/Struct_InventorySlotData Structure") (`Chest Slot To Update` :type "Object Object Reference"))
  (bind (_isempty _itemdata) (break `/Game/Inventory/Blueprint/Inventory/Struct_InventorySlotData` `New Slot Data`))
  (bind _inventoryslots (`self.InventorySlots`))
  (bind _returnvalue (`KismetArrayLibrary.Array_Find` _inventoryslots (`/Game/Inventory/Blueprint/UI/WBP_InventorySlot.Inventory Slot Data` `Slot To Update`)))
  (`|ExecutionSequence`
    (:`then_0`
      (if (!= _returnvalue -1)
        (setmembers `/Game/Inventory/Blueprint/Inventory/Struct_InventorySlotData` :`StructRef` (`|GetArrayItem` _inventoryslots _returnvalue) :`isEmpty` _isempty :`ItemData` _itemdata))
      (bind _structout (setmembers `/Game/Inventory/Blueprint/Inventory/Struct_InventorySlotData` :`StructRef` (`/Game/Inventory/Blueprint/UI/WBP_InventorySlot.Inventory Slot Data` `Slot To Update`) :`isEmpty` _isempty :`ItemData` _itemdata))
      (`/Game/Inventory/Blueprint/UI/WBP_InventorySlot.Init/Update Slot` (`local.Slot To Update`) _structout))))