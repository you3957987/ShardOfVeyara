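; BP_ItemMaster is a world item pickup that the farmer character collects by touching it.
; On BeginPlay it initializes its item data, then enables query-only collision on its sphere after a configurable delay.
; When a BP_Farmer overlaps the sphere, it adds its ID and amount to that farmer's inventory component.
; Only a successful add shows a HUD notification and destroys the actor.
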(event `self.ReceiveBeginPlay`
  (`self.Initialize Item Data Structure`)
  (`KismetSystemLibrary.Delay` (`self.EnableDelay`))
  (`PrimitiveComponent.SetCollisionEnabled` (`self.Sphere`) "QueryOnly"))

(event `self.Sphere.OnComponentBeginOverlap`
  (params (OverlappedComponent :type "PrimitiveComponent Object Reference") (OtherActor :type "Actor Object Reference") (OtherComp :type "PrimitiveComponent Object Reference") (OtherBodyIndex :type Integer) (bFromSweep :type Boolean) (SweepResult :type "HitResult Structure (by ref)"))
  (bind _asbp_farmer (cast `/Game/HYH/Blueprints/BP_Farmer` OtherActor))
  (`|ExecutionSequence`
    (:`then_0`
      (bind _success_ (`/Game/Inventory/Blueprint/Inventory/BPAC_InventoryComponent.Add Item` (`/Game/HYH/Blueprints/BP_Farmer.BPAC_InventoryComponent` _asbp_farmer) (`self.ItemID`) (`self.Amount`)))
      (if _success_
        (`/Game/Inventory/Blueprint/UI/WBP_PlayerHUD.Add Item Notification` (`/Game/HYH/Blueprints/BP_Farmer.Player HUD Ref` _asbp_farmer) (`self.Item Data Struct`) (`self.Amount`))
        (`self.K2_DestroyActor`)))))

(fn `UserConstructionScript`)