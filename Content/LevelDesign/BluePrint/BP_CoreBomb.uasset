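; BP_CoreBomb is a hidden pit with a core that appears after the player approaches and serves as a level transition.
; BeginPlay hides Hole and Core0 and disables their collision.
; Player overlap with Box1 waits five seconds, then plays a sound and reveals both.
; Box plays a sound on any overlap and, for the player, stores TeleTag in BP_GameInstance and opens Level, independent of pit visibility.
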(event `Visible`
  ; 구덩이 가시성 여부
  (`SceneComponent.SetVisibility` (`self.Hole`) true false)
  (`SceneComponent.SetVisibility` (`self.Core_0`) true false)
  (`PrimitiveComponent.SetCollisionEnabled` (`self.Hole`) "QueryOnly")
  (`PrimitiveComponent.SetCollisionEnabled` (`self.Core_0`) "QueryOnly"))

(event `Invisible`
  ; 구덩이 가시성 여부
  (`SceneComponent.SetVisibility` (`self.Hole`) false false)
  (`SceneComponent.SetVisibility` (`self.Core_0`) false false)
  (`PrimitiveComponent.SetCollisionEnabled` (`self.Hole`) "NoCollision")
  (`PrimitiveComponent.SetCollisionEnabled` (`self.Core_0`) "NoCollision"))

(event `self.ReceiveBeginPlay`
  ; 구덩이 불러오기
  (`self.Invisible`))

(event `self.Box 1.OnComponentBeginOverlap`
  (params (OverlappedComponent :type "PrimitiveComponent Object Reference") (OtherActor :type "Actor Object Reference") (OtherComp :type "PrimitiveComponent Object Reference") (OtherBodyIndex :type Integer) (bFromSweep :type Boolean) (SweepResult :type "HitResult Structure (by ref)"))
  ; 구덩이 불러오기
  (if (== OtherActor (`GameplayStatics.GetPlayerPawn` 0))
    (`KismetSystemLibrary.Delay` 5.0)
    (`AudioComponent.Play` (`self.Audio`) 0.0)
    (`self.Visible`)))

(event `self.Box.OnComponentBeginOverlap`
  (params (OverlappedComponent :type "PrimitiveComponent Object Reference") (OtherActor :type "Actor Object Reference") (OtherComp :type "PrimitiveComponent Object Reference") (OtherBodyIndex :type Integer) (bFromSweep :type Boolean) (SweepResult :type "HitResult Structure (by ref)"))
  ; 구덩이 진입 시 레벨이동
  (`AudioComponent.Play` (`self.Audio1`) 0.0)
  (if (== OtherActor (`GameplayStatics.GetPlayerPawn` 0))
    (bind _asbp_game_instance (cast `/Game/LevelDesign/BluePrint/BP_GameInstance` (`GameplayStatics.GetGameInstance`)))
    (set `/Game/LevelDesign/BluePrint/BP_GameInstance.Teleportation Tag` (`self.Tele Tag`) _asbp_game_instance)
    (`GameplayStatics.OpenLevelBySoftObjectPtr` (`self.Level`))))

(fn `UserConstructionScript`)