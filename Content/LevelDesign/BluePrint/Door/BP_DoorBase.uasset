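; Base interactable door that a BP_Farmer can open and close, with an "열기"/"닫기" (open/close) prompt shown through the AGSD player controller.
; A box trigger adds and removes the door from the farmer's interactable list on overlap.
; Interact alternates open and close through a FlipFlop, playing or reversing a timeline that rotates the door up to 90 degrees.
; Box collision is off during the swing and returns to query-only when it finishes.
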(event `DoorOpen`
  (set `self.New Text` "닫기")
  (bind (_direction `_새_트랙_0`) (`Timeline|Door_Ani` :!via `PlayFromStart` :!label _label)
    (:`Update`
      (`SceneComponent.K2_SetRelativeRotation` (`self.Door`) (`KismetMathLibrary.RLerp` (struct) (struct :`Yaw` 90.0) `_새_트랙_0` true) false false))
    (:`Finished`
      (`PrimitiveComponent.SetCollisionEnabled` (`self.Box`) "QueryOnly"))))

(event `DoorClose`
  (set `self.New Text` "열기")
  (goto _label :!via `Reverse`))

(event `self.Interact`
  (params (player :type "AGSDCharacter Object Reference"))
  (`PrimitiveComponent.SetCollisionEnabled` (`self.Box`) "NoCollision")
  (`/Engine/EditorBlueprintResources/StandardMacros.FlipFlop`
    (:`A`
      (`self.DoorOpen`))
    (:`B`
      (`self.DoorClose`))))

(event `self.Box.OnComponentBeginOverlap`
  (params (OverlappedComponent :type "PrimitiveComponent Object Reference") (OtherActor :type "Actor Object Reference") (OtherComp :type "PrimitiveComponent Object Reference") (OtherBodyIndex :type Integer) (bFromSweep :type Boolean) (SweepResult :type "HitResult Structure (by ref)"))
  (bind _asbp_farmer (cast `/Game/HYH/Blueprints/BP_Farmer` OtherActor))
  (`AGSDCharacter.AddInteractableActor` _asbp_farmer self))

(event `self.Box.OnComponentEndOverlap`
  (params (OverlappedComponent :type "PrimitiveComponent Object Reference") (OtherActor :type "Actor Object Reference") (OtherComp :type "PrimitiveComponent Object Reference") (OtherBodyIndex :type Integer))
  (bind _asbp_farmer (cast `/Game/HYH/Blueprints/BP_Farmer` OtherActor))
  (`AGSDCharacter.RemoveInteractableActor` _asbp_farmer self))

(event `self.ShowWidget`
  (params (player :type "Character Object Reference"))
  (bind _asagsdplayer_controller (cast `AGSDPlayerController` (`GameplayStatics.GetPlayerController` 0)))
  (`AGSDPlayerController.ShowInteractionWidget` _asagsdplayer_controller (`self.New Text`)))

(fn `CanInteract`
  (params (player :type "AGSDCharacter Object Reference"))
  (returns (ReturnValue :type Boolean))
  (return true))

(fn `UserConstructionScript`)