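; Interactable switch, shown with a configurable book mesh, that reports its activation to a linked door.
; Overlapping the Box registers it as interactable with BP_Farmer, and leaving unregisters it; a widget prompt is shown through the player controller.
; Interacting calls SwitchesActivated on DoorToActivate, removes the interactable from the player, then disables Box collision and hides only the Box, so the switch is single-use.
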(event `self.ReceiveBeginPlay`
  (`StaticMeshComponent.SetStaticMesh` (`self.Book`) (`self.Book Object`)))

(event `self.ShowWidget`
  (params (player :type "Character Object Reference"))
  (bind _asagsdplayer_controller (cast `AGSDPlayerController` (`GameplayStatics.GetPlayerController` 0)))
  (`AGSDPlayerController.ShowInteractionWidget` _asagsdplayer_controller (`self.New Text`)))

(event `self.Interact`
  (params (player :type "AGSDCharacter Object Reference"))
  (bind _box (`self.Box`))
  (`AGSDCharacter.RemoveInteractableActor` player null)
  (`/Game/LevelDesign/BluePrint/Machine/BP_Generator_1.SwitchesActivated` (`self.DoorToActivate`))
  (`PrimitiveComponent.SetCollisionEnabled` _box "NoCollision")
  (`SceneComponent.SetVisibility` _box false false))

(event `self.Box.OnComponentBeginOverlap`
  (params (OverlappedComponent :type "PrimitiveComponent Object Reference") (OtherActor :type "Actor Object Reference") (OtherComp :type "PrimitiveComponent Object Reference") (OtherBodyIndex :type Integer) (bFromSweep :type Boolean) (SweepResult :type "HitResult Structure (by ref)"))
  (bind _asbp_farmer (cast `/Game/HYH/Blueprints/BP_Farmer` OtherActor))
  (`AGSDCharacter.AddInteractableActor` _asbp_farmer null))

(event `self.Box.OnComponentEndOverlap`
  (params (OverlappedComponent :type "PrimitiveComponent Object Reference") (OtherActor :type "Actor Object Reference") (OtherComp :type "PrimitiveComponent Object Reference") (OtherBodyIndex :type Integer))
  (bind _asbp_farmer (cast `/Game/HYH/Blueprints/BP_Farmer` OtherActor))
  (`AGSDCharacter.RemoveInteractableActor` _asbp_farmer null))

(fn `CanInteract`
  (params (player :type "AGSDCharacter Object Reference"))
  (returns (ReturnValue :type Boolean))
  (return true))

(fn `UserConstructionScript`)