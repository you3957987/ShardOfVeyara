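; BP_SwitchDoor_2 is a pressure-switch-driven door variant whose Box appears, rather than disappears, when enough switches are active.
; It starts with the Box hidden and collision disabled.
; SwitchesActivated and SwitchesDeactivated adjust an active-switch count and compare it to the required number.
; Meeting the threshold shows the Box with query-only collision; falling below hides it and disables collision again.
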(event `self.ReceiveBeginPlay`
  (bind _box (`self.Box`))
  (`SceneComponent.SetVisibility` _box false false)
  (`PrimitiveComponent.SetCollisionEnabled` _box "NoCollision"))

(event `SwitchesActivated`
  (bind _box (`self.Box`))
  (`/Engine/EditorBlueprintResources/StandardMacros.IncrementInt` (`self.PressureSwitchesActive`)
    (:`  `
      (if (>= (`self.PressureSwitchesActive`) (`self.PressureSwitchesNeeded`))
        (`SceneComponent.SetVisibility` _box true false :!label _label)
        (`PrimitiveComponent.SetCollisionEnabled` _box "QueryOnly")
        (else
          (`SceneComponent.SetVisibility` _box false false :!label _label_2)
          (`PrimitiveComponent.SetCollisionEnabled` _box "NoCollision"))))))

(event `SwitchesDeactivated`
  (`/Engine/EditorBlueprintResources/StandardMacros.DecrementInt` (`self.PressureSwitchesActive`)
    (:`  `
      (if (>= (`self.PressureSwitchesActive`) (`self.PressureSwitchesNeeded`))
        (goto _label)
        (else
          (goto _label_2))))))

(fn `UserConstructionScript`)