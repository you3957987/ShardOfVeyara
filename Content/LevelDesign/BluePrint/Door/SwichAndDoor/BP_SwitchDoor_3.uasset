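; BP_SwitchDoor_3 is a door that moves along Z when enough pressure switches are active.
; Activation and deactivation events raise or lower a count and compare it to the required number, playing or reversing the DoorActivation timeline that drives the door's relative location.
; Activation plays the timeline at or above the threshold, while deactivation plays it only strictly above, so dropping to exactly the required count reverses the door.
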(event `SwitchesActivated`
  (`/Engine/EditorBlueprintResources/StandardMacros.IncrementInt` (`self.PressureSwitchesActive`)
    (:`  `
      (if (>= (`self.PressureSwitchesActive`) (`self.PressureSwitchesNeeded`))
        (bind (_direction _newtrack_0) (`Timeline|DoorActivation` :!label _label)
          (:`Update`
            (`SceneComponent.K2_SetRelativeLocation` (`self.Door`) (`KismetMathLibrary.MakeVector` 0.0 0.0 _newtrack_0) false false)))
        (else
          (goto _label :!via `Reverse`))))))

(event `SwitchesDeactivated`
  (`/Engine/EditorBlueprintResources/StandardMacros.DecrementInt` (`self.PressureSwitchesActive`)
    (:`  `
      (if (> (`self.PressureSwitchesActive`) (`self.PressureSwitchesNeeded`))
        (goto _label)
        (else
          (goto _label :!via `Reverse`))))))

(fn `UserConstructionScript`)