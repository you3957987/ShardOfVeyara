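; Interactable double dungeon door that a BP_Farmer opens on interaction and that closes when the farmer leaves its trigger box.
; Box overlaps add or remove the door as the farmer's interactable; Interact also removes it, then opens the door.
; A single timeline swings both leaves 90 degrees in opposite directions and plays in reverse to close.
; CanInteract always allows use, and ShowWidget displays the interaction prompt through the AGSD player controller.
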(event `DoorOpen`
  ; 문 열리는 애니메이션
  (bind (_direction `_새_트랙_0`) (`Timeline|Door_Ani` :!label _label)
    (:`Update`
      (`SceneComponent.K2_SetRelativeRotation` (`self.Door_1`) (`KismetMathLibrary.RLerp` (struct) (struct :`Yaw` 90.0) `_새_트랙_0` true) false false)
      (`SceneComponent.K2_SetRelativeRotation` (`self.Door_2`) (`KismetMathLibrary.RLerp` (struct) (struct :`Yaw` -90.0) `_새_트랙_0` true) false false))))

(event `DoorClose`
  ; 문 열리는 애니메이션
  (goto _label :!via `Reverse`))

(event `self.Interact`
  (params (player :type "AGSDCharacter Object Reference"))
  ; 콜리젼 충돌 시 열고 닫힘
  (`AGSDCharacter.RemoveInteractableActor` player self)
  (`self.DoorOpen`))

(event `self.Box.OnComponentEndOverlap`
  (params (OverlappedComponent :type "PrimitiveComponent Object Reference") (OtherActor :type "Actor Object Reference") (OtherComp :type "PrimitiveComponent Object Reference") (OtherBodyIndex :type Integer))
  ; 콜리젼 충돌 시 열고 닫힘
  (bind _asbp_farmer (cast `/Game/HYH/Blueprints/BP_Farmer` OtherActor))
  (`AGSDCharacter.RemoveInteractableActor` _asbp_farmer self)
  (`self.DoorClose`))

(event `self.Box.OnComponentBeginOverlap`
  (params (OverlappedComponent :type "PrimitiveComponent Object Reference") (OtherActor :type "Actor Object Reference") (OtherComp :type "PrimitiveComponent Object Reference") (OtherBodyIndex :type Integer) (bFromSweep :type Boolean) (SweepResult :type "HitResult Structure (by ref)"))
  ; 콜리젼 충돌 시 열고 닫힘
  (bind _asbp_farmer (cast `/Game/HYH/Blueprints/BP_Farmer` OtherActor))
  (`AGSDCharacter.AddInteractableActor` _asbp_farmer self))

(event `self.ShowWidget`
  (params (player :type "Character Object Reference"))
  ; 콜리젼 충돌 시 열고 닫힘
  (bind _asagsdplayer_controller (cast `AGSDPlayerController` (`GameplayStatics.GetPlayerController` 0)))
  (`AGSDPlayerController.ShowInteractionWidget` _asagsdplayer_controller (`self.New Text`)))

(fn `CanInteract`
  (params (player :type "AGSDCharacter Object Reference"))
  (returns (ReturnValue :type Boolean))
  (return true))

(fn `UserConstructionScript`)