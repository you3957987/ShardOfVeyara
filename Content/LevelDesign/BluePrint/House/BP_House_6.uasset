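; BP_House_6 is a house actor with a door the player can open and close when nearby.
; Overlapping the Box component enables player input on the actor, and ending the overlap disables it, with no filter on the overlapping actor.
; The IA_Interaction action alternates through a FlipFlop between DoorOpen and DoorClose.
; These play or reverse the Door_Ani timeline, which lerps the door's relative yaw or roll rotation to swing it.
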(event `DoorOpen`
  (bind (_direction `_새_트랙_0`) (`Timeline|Door_Ani` :!via `PlayFromStart` :!label _label)
    (:`Update`
      (`SceneComponent.K2_SetRelativeRotation` (`self.Door`) (`KismetMathLibrary.RLerp` (struct) (struct :`Yaw` 90.0) `_새_트랙_0` true) false false))))

(event `DoorClose`
  (goto _label :!via `Reverse`))

(event `EnhancedInput|/Game/HYH/Input/IA_Interaction`
  (params (ActionValue :type Boolean) (ElapsedSeconds :type "Float (double-precision)") (TriggeredSeconds :type "Float (double-precision)") (InputAction :type "InputAction Object Reference" :default "/Game/HYH/Input/IA_Interaction.IA_Interaction"))
  (:`Triggered`
    (`/Engine/EditorBlueprintResources/StandardMacros.FlipFlop`
      (:`A`
        (`self.DoorOpen`))
      (:`B`
        (`self.DoorClose`)))))

(event `self.Box.OnComponentBeginOverlap`
  (params (OverlappedComponent :type "PrimitiveComponent Object Reference") (OtherActor :type "Actor Object Reference") (OtherComp :type "PrimitiveComponent Object Reference") (OtherBodyIndex :type Integer) (bFromSweep :type Boolean) (SweepResult :type "HitResult Structure (by ref)"))
  (`self.EnableInput` (`GameplayStatics.GetPlayerController` 0)))

(event `self.Box.OnComponentEndOverlap`
  (params (OverlappedComponent :type "PrimitiveComponent Object Reference") (OtherActor :type "Actor Object Reference") (OtherComp :type "PrimitiveComponent Object Reference") (OtherBodyIndex :type Integer))
  (`self.DisableInput` (`GameplayStatics.GetPlayerController` 0)))

(fn `UserConstructionScript`)