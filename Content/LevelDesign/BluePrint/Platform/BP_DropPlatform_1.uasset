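; BP_DropPlatform_1 is a spinning circular platform that falls after the player enters its overlap.
; Tick continuously applies a local rotation to the floor mesh.
; When the first player character begins overlapping the actor, the core switches to a second material as a visible cue.
; After a configurable delay, the floor enables physics simulation to drop.
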(event `self.ReceiveTick`
  (params (DeltaSeconds :type "Float (single-precision)"))
  (`SceneComponent.K2_AddLocalRotation` (`self.Circle_Floor_1`) (`self.Spin Rotation`) false false))

(event `self.ReceiveActorBeginOverlap`
  (params (OtherActor :type "Actor Object Reference"))
  (if (== (`GameplayStatics.GetPlayerCharacter` 0) OtherActor)
    (`PrimitiveComponent.SetMaterial` (`self.Circle_Floor_Core_1`) 0 "/Game/LevelDesign/Materials/M_Create/M_Core2.M_Core2")
    (`KismetSystemLibrary.Delay` (`self.Delay Time`))
    (`PrimitiveComponent.SetSimulatePhysics` (`self.Circle_Floor_1`) true)))

(fn `UserConstructionScript`)