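; BP_MovingPlatform_1 is a moving platform with a spinning circular floor and its own audio.
; The construction script sets InterpToMovement's two relative control points from Location01 and Location02, and its travel time from Duration.
; BeginPlay starts the audio, and Tick adds SpinRotation to CircleFloor1's local rotation each frame without delta-time scaling, so spin speed depends on frame rate.
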(event `self.ReceiveBeginPlay`
  (`AudioComponent.Play` (`self.Audio`) 0.0))

(event `self.ReceiveTick`
  (params (DeltaSeconds :type "Float (single-precision)"))
  (`SceneComponent.K2_AddLocalRotation` (`self.Circle_Floor_1`) (`self.Spin Rotation`) false false))

(fn `UserConstructionScript`
  (bind _interptomovement (`self.InterpToMovement`))
  (set `InterpToMovementComponent.ControlPoints` (`|MakeArray` (make `InterpControlPoint` (`self.Location01`)) (make `InterpControlPoint` (`self.Location02`))) _interptomovement)
  (set `InterpToMovementComponent.Duration` (`self.Duration`) _interptomovement))