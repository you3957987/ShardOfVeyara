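; BP_JumpingPlatform_1 is a jump pad platform that launches the player when they step onto it.
; On actor overlap with the player character, it plays its audio and adds an impulse to the character's movement component.
; The impulse follows the Arrow component's forward vector scaled by JumpPower, applied as a velocity change so mass is ignored.
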(event `self.ReceiveActorBeginOverlap`
  (params (OtherActor :type "Actor Object Reference"))
  (if (== (`GameplayStatics.GetPlayerCharacter` 0) OtherActor)
    (`AudioComponent.Play` (`self.Audio`) 0.0)
    (`CharacterMovementComponent.AddImpulse` (`Character.CharacterMovement` (`GameplayStatics.GetPlayerCharacter` 0)) (* (`SceneComponent.GetForwardVector` (`self.Arrow`)) (`self.Jump Power`)) true)))

(fn `UserConstructionScript`)