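; Platform actor that travels along a referenced spline actor's path, starting automatically at BeginPlay.
; MoveObject applies the configured mesh to its Cube, then plays the Move timeline at a rate of 1/Time.
; Each update maps the timeline alpha to distance along the spline and sets the world location there.
; Rotation is always sampled at the spline's start in local space, so it does not follow the curve.
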(event `self.ReceiveBeginPlay`
  (`self.Move Object`))

(event `Move Object`
  (bind _spline (`/Game/LevelDesign/BluePrint/Platform/BP_PlatformSpline.Spline` (`self.SplineToFollow`)))
  (`StaticMeshComponent.SetStaticMesh` (`self.Cube`) (`self.Object`))
  (`TimelineComponent.SetPlayRate` (`self.Move`) (/ 1.0 (`self.Time`)))
  (bind (_direction _newtrack_0) (`Timeline|Move`)
    (:`Update`
      (`self.K2_SetActorLocationAndRotation` (`SplineComponent.GetLocationAtDistanceAlongSpline` _spline (`KismetMathLibrary.Lerp` 0.0 (`SplineComponent.GetSplineLength` _spline) _newtrack_0) "World") (`SplineComponent.GetRotationAtDistanceAlongSpline` _spline 0.0 "Local")))))

(fn `UserConstructionScript`)