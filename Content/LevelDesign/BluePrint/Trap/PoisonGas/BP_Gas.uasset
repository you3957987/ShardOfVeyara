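; BP_Gas is a poison gas trap that periodically damages a BP_Farmer inside its GasBox.
; Overlap begin starts a looping damage timer on the stored farmer, and overlap end clears it.
; GasSwitchesOff and GasSwitchesOn adjust an active pressure-switch count against the required number, toggling GasBox visibility and collision.
; The threshold test is inclusive on increment but strict on decrement.
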(event `Gas Switches Off`
  (bind _gas_box (`self.Gas Box`))
  (`/Engine/EditorBlueprintResources/StandardMacros.IncrementInt` (`self.PressureSwitchesActive`)
    (:`  `
      (if (>= (`self.PressureSwitchesActive`) (`self.PressureSwitchesNeeded`))
        (`SceneComponent.SetVisibility` _gas_box false false :!label _label)
        (`PrimitiveComponent.SetCollisionEnabled` _gas_box "NoCollision")
        (else
          (`SceneComponent.SetVisibility` _gas_box true false :!label _label_2)
          (`PrimitiveComponent.SetCollisionEnabled` _gas_box "QueryOnly"))))))

(event `Gas Switches On`
  (`/Engine/EditorBlueprintResources/StandardMacros.DecrementInt` (`self.PressureSwitchesActive`)
    (:`  `
      (if (> (`self.PressureSwitchesActive`) (`self.PressureSwitchesNeeded`))
        (goto _label)
        (else
          (goto _label_2))))))

(event `Apply Gas Damage`
  ; 독가스 체력깎임
  (`GameplayStatics.ApplyDamage` (stale `self.Gas Box.OnComponentBeginOverlap` _asbp_farmer) (`self.Damage`)))

(event `self.Gas Box.OnComponentBeginOverlap`
  (params (OverlappedComponent :type "PrimitiveComponent Object Reference") (OtherActor :type "Actor Object Reference") (OtherComp :type "PrimitiveComponent Object Reference") (OtherBodyIndex :type Integer) (bFromSweep :type Boolean) (SweepResult :type "HitResult Structure (by ref)"))
  ; 독가스 체력깎임
  (bind _asbp_farmer (cast `/Game/HYH/Blueprints/BP_Farmer` OtherActor))
  (bind _returnvalue (`KismetSystemLibrary.K2_SetTimerDelegate` (delegate `Apply Gas Damage`) (`self.Damage Time`) true))
  (set `self.GasTimerHandle` _returnvalue))

(event `self.Gas Box.OnComponentEndOverlap`
  (params (OverlappedComponent :type "PrimitiveComponent Object Reference") (OtherActor :type "Actor Object Reference") (OtherComp :type "PrimitiveComponent Object Reference") (OtherBodyIndex :type Integer))
  ; 독가스 체력깎임
  (cast `/Game/HYH/Blueprints/BP_Farmer` OtherActor)
  (`KismetSystemLibrary.K2_ClearAndInvalidateTimerHandle` (`self.GasTimerHandle`)))

(fn `UserConstructionScript`)