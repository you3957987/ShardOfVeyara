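; Fire trap that stays hidden until the farmer (BP_Farmer) walks into its DeathZone, then kills them.
; BeginPlay hides NSFire and Ground16 and turns off the fire's collision.
; On overlap it reveals both, sets the fire to query-only collision, then applies lethal damage after a short delay without rechecking the overlap.
; Nothing hides the trap again once triggered.
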(event `self.ReceiveBeginPlay`
  (bind _ns_fire (`self.NS_Fire`))
  (`SceneComponent.SetVisibility` _ns_fire false false)
  (`PrimitiveComponent.SetCollisionEnabled` _ns_fire "NoCollision")
  (`SceneComponent.SetVisibility` (`self.Ground_16`) false false))

(event `self.Death Zone.OnComponentBeginOverlap`
  (params (OverlappedComponent :type "PrimitiveComponent Object Reference") (OtherActor :type "Actor Object Reference") (OtherComp :type "PrimitiveComponent Object Reference") (OtherBodyIndex :type Integer) (bFromSweep :type Boolean) (SweepResult :type "HitResult Structure (by ref)"))
  (bind _ns_fire (`self.NS_Fire`))
  (bind _asbp_farmer (cast `/Game/HYH/Blueprints/BP_Farmer` OtherActor))
  (`SceneComponent.SetVisibility` _ns_fire true false)
  (`PrimitiveComponent.SetCollisionEnabled` _ns_fire "QueryOnly")
  (`SceneComponent.SetVisibility` (`self.Ground_16`) true false)
  (`KismetSystemLibrary.Delay` 0.2)
  (`GameplayStatics.ApplyDamage` _asbp_farmer 100000.0))

(fn `UserConstructionScript`)