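; BP_Drop is a falling-rock trap that can damage BP_Farmer.
; When the farmer enters the Box trigger, a short delay runs before physics is enabled on the Rock so it can drop.
; A separate Sphere overlap applies the Damage value to the farmer, then hides the Sphere and disables its collision so it stops registering hits.
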(event `self.Box.OnComponentBeginOverlap`
  (params (OverlappedComponent :type "PrimitiveComponent Object Reference") (OtherActor :type "Actor Object Reference") (OtherComp :type "PrimitiveComponent Object Reference") (OtherBodyIndex :type Integer) (bFromSweep :type Boolean) (SweepResult :type "HitResult Structure (by ref)"))
  (cast `/Game/HYH/Blueprints/BP_Farmer` OtherActor)
  (`KismetSystemLibrary.Delay` 0.5)
  (`PrimitiveComponent.SetSimulatePhysics` (`self.Rock`) true))

(event `self.Sphere.OnComponentBeginOverlap`
  (params (OverlappedComponent :type "PrimitiveComponent Object Reference") (OtherActor :type "Actor Object Reference") (OtherComp :type "PrimitiveComponent Object Reference") (OtherBodyIndex :type Integer) (bFromSweep :type Boolean) (SweepResult :type "HitResult Structure (by ref)"))
  (bind _sphere (`self.Sphere`))
  (bind _asbp_farmer (cast `/Game/HYH/Blueprints/BP_Farmer` OtherActor))
  (`GameplayStatics.ApplyDamage` _asbp_farmer (`self.Damage`))
  (`SceneComponent.SetVisibility` _sphere false false)
  (`PrimitiveComponent.SetCollisionEnabled` _sphere "NoCollision"))

(fn `UserConstructionScript`)