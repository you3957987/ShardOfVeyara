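; BP_FoldingTrap_1 is a level trap that folds open after a BP_Farmer stands in its Box trigger for TrapOpeningTime.
; Entering the box starts a timer that plays the Foldering timeline, which lerps the Folder component's roll from 0 to 90 degrees.
; Leaving the box clears the pending timer and reverses the timeline to swing the Folder back.
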(event `self.Box.OnComponentBeginOverlap`
  (params (OverlappedComponent :type "PrimitiveComponent Object Reference") (OtherActor :type "Actor Object Reference") (OtherComp :type "PrimitiveComponent Object Reference") (OtherBodyIndex :type Integer) (bFromSweep :type Boolean) (SweepResult :type "HitResult Structure (by ref)"))
  (cast `/Game/HYH/Blueprints/BP_Farmer` OtherActor)
  (bind _returnvalue (`KismetSystemLibrary.K2_SetTimerDelegate` (delegate `Folding`) (`self.TrapOpeningTime`)))
  (set `self.Timer` _returnvalue))

(event `Folding`
  (bind (_direction _newtrack_0) (`Timeline|Foldering`)
    (:`Update`
      (`SceneComponent.K2_SetRelativeRotation` (`self.Folder`) (`KismetMathLibrary.MakeRotator` (`KismetMathLibrary.Lerp` 0.0 90.0 _newtrack_0)) false false))))

(event `self.Box.OnComponentEndOverlap`
  (params (OverlappedComponent :type "PrimitiveComponent Object Reference") (OtherActor :type "Actor Object Reference") (OtherComp :type "PrimitiveComponent Object Reference") (OtherBodyIndex :type Integer))
  (cast `/Game/HYH/Blueprints/BP_Farmer` OtherActor)
  (`KismetSystemLibrary.K2_ClearAndInvalidateTimerHandle` (`self.Timer`))
  (`TimelineComponent.Reverse` (`self.Foldering`)))

(fn `UserConstructionScript`)