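; BP_TowerCraneButton_1 is a machine control with left and right buttons that rotate a tower crane.
; Both trigger components start hidden with collision off until UseEnergy shows them and enables query collision.
; A BP_Farmer overlapping a trigger starts the Crane rotating that way and turns the button light blue; leaving stops rotation and turns it red.
; CanInteract always returns false, so overlaps alone drive the crane.
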(event `self.ReceiveBeginPlay`
  (bind _right (`self.Right`))
  (`SceneComponent.SetVisibility` _right false false)
  (`SceneComponent.SetVisibility` (`self.Left`) false false)
  (`PrimitiveComponent.SetCollisionEnabled` _right "NoCollision")
  (`PrimitiveComponent.SetCollisionEnabled` (`self.Left`) "NoCollision"))

(event `Use Energy`
  (bind _right (`self.Right`))
  (`SceneComponent.SetVisibility` _right true false)
  (`SceneComponent.SetVisibility` (`self.Left`) true false)
  (`PrimitiveComponent.SetCollisionEnabled` _right "QueryOnly")
  (`PrimitiveComponent.SetCollisionEnabled` (`self.Left`) "QueryOnly"))

(event `self.Left.OnComponentBeginOverlap`
  (params (OverlappedComponent :type "PrimitiveComponent Object Reference") (OtherActor :type "Actor Object Reference") (OtherComp :type "PrimitiveComponent Object Reference") (OtherBodyIndex :type Integer) (bFromSweep :type Boolean) (SweepResult :type "HitResult Structure (by ref)"))
  ; 크레인 작동 버튼
  (cast `/Game/HYH/Blueprints/BP_Farmer` OtherActor)
  (`/Game/LevelDesign/BluePrint/Machine/BP_TowerCrane_1.Rotate Left` (`self.Crane`))
  (`PrimitiveComponent.SetMaterial` (`self.Left Button`) 0 "/Game/LevelDesign/Materials/M_Create/M_BlueLight1.M_BlueLight1"))

(event `self.Left.OnComponentEndOverlap`
  (params (OverlappedComponent :type "PrimitiveComponent Object Reference") (OtherActor :type "Actor Object Reference") (OtherComp :type "PrimitiveComponent Object Reference") (OtherBodyIndex :type Integer))
  ; 크레인 작동 버튼
  (cast `/Game/HYH/Blueprints/BP_Farmer` OtherActor)
  (`/Game/LevelDesign/BluePrint/Machine/BP_TowerCrane_1.Rotate Stop` (`self.Crane`))
  (`PrimitiveComponent.SetMaterial` (`self.Left Button`) 0 "/Game/LevelDesign/Materials/M_Create/M_RedLight.M_RedLight"))

(event `self.Right.OnComponentBeginOverlap`
  (params (OverlappedComponent :type "PrimitiveComponent Object Reference") (OtherActor :type "Actor Object Reference") (OtherComp :type "PrimitiveComponent Object Reference") (OtherBodyIndex :type Integer) (bFromSweep :type Boolean) (SweepResult :type "HitResult Structure (by ref)"))
  ; 크레인 작동 버튼
  (cast `/Game/HYH/Blueprints/BP_Farmer` OtherActor)
  (`/Game/LevelDesign/BluePrint/Machine/BP_TowerCrane_1.Rotate Right` (`self.Crane`))
  (`PrimitiveComponent.SetMaterial` (`self.Right Button`) 0 "/Game/LevelDesign/Materials/M_Create/M_BlueLight1.M_BlueLight1"))

(event `self.Right.OnComponentEndOverlap`
  (params (OverlappedComponent :type "PrimitiveComponent Object Reference") (OtherActor :type "Actor Object Reference") (OtherComp :type "PrimitiveComponent Object Reference") (OtherBodyIndex :type Integer))
  ; 크레인 작동 버튼
  (cast `/Game/HYH/Blueprints/BP_Farmer` OtherActor)
  (`/Game/LevelDesign/BluePrint/Machine/BP_TowerCrane_1.Rotate Stop` (`self.Crane`))
  (`PrimitiveComponent.SetMaterial` (`self.Right Button`) 0 "/Game/LevelDesign/Materials/M_Create/M_RedLight.M_RedLight"))

(fn `CanInteract`
  (params (player :type "AGSDCharacter Object Reference"))
  (returns (ReturnValue :type Boolean))
  (return false))

(fn `UserConstructionScript`)