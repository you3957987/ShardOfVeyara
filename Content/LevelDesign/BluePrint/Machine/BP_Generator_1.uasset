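; Generator machine that becomes usable once enough fuses or pressure switches are active.
; Activate and deactivate events adjust a counter, showing the Box and enabling query collision at the required threshold, otherwise hiding and disabling it.
; Box overlaps register the generator as an interactable on BP_Farmer.
; ShowWidget displays the prompt through AGSDPlayerController, and Interact calls UseEnergy on its target, though CanInteract always returns false.
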(event `self.ReceiveBeginPlay`
  (bind _box (`self.Box`))
  ; 퓨즈 작동 시 발전기 사용가능
  (`SceneComponent.SetVisibility` _box false false)
  (`PrimitiveComponent.SetCollisionEnabled` _box "NoCollision"))

(event `Generator Activated`
  (bind _box (`self.Box`))
  ; 퓨즈 작동 시 발전기 사용가능
  (`/Engine/EditorBlueprintResources/StandardMacros.IncrementInt` (`self.PressureSwitchesActive`)
    (:`  `
      (if (>= (`self.PressureSwitchesActive`) (`self.PressureSwitchesNeeded`))
        (`SceneComponent.SetVisibility` _box true false :!label _label)
        (`PrimitiveComponent.SetCollisionEnabled` _box "QueryOnly")
        (else
          (`SceneComponent.SetVisibility` _box false false :!label _label_2)
          (`PrimitiveComponent.SetCollisionEnabled` _box "NoCollision"))))))

(event `Generator Deactivated`
  ; 퓨즈 작동 시 발전기 사용가능
  (`/Engine/EditorBlueprintResources/StandardMacros.DecrementInt` (`self.PressureSwitchesActive`)
    (:`  `
      (if (>= (`self.PressureSwitchesActive`) (`self.PressureSwitchesNeeded`))
        (goto _label)
        (else
          (goto _label_2))))))

(event `self.Box.OnComponentBeginOverlap`
  (params (OverlappedComponent :type "PrimitiveComponent Object Reference") (OtherActor :type "Actor Object Reference") (OtherComp :type "PrimitiveComponent Object Reference") (OtherBodyIndex :type Integer) (bFromSweep :type Boolean) (SweepResult :type "HitResult Structure (by ref)"))
  (bind _asbp_farmer (cast `/Game/HYH/Blueprints/BP_Farmer` OtherActor))
  (`AGSDCharacter.AddInteractableActor` _asbp_farmer self))

(event `self.Box.OnComponentEndOverlap`
  (params (OverlappedComponent :type "PrimitiveComponent Object Reference") (OtherActor :type "Actor Object Reference") (OtherComp :type "PrimitiveComponent Object Reference") (OtherBodyIndex :type Integer))
  (bind _asbp_farmer (cast `/Game/HYH/Blueprints/BP_Farmer` OtherActor))
  (`AGSDCharacter.RemoveInteractableActor` _asbp_farmer self))

(event `self.ShowWidget`
  (params (player :type "Character Object Reference"))
  (bind _asagsdplayer_controller (cast `AGSDPlayerController` (`GameplayStatics.GetPlayerController` 0)))
  (`AGSDPlayerController.ShowInteractionWidget` _asagsdplayer_controller (`self.New Text`)))

(event `self.Interact`
  (params (player :type "AGSDCharacter Object Reference"))
  (`/Game/LevelDesign/BluePrint/Machine/BP_TowerCraneButton_1.Use Energy` (`self.Target`)))

(fn `CanInteract`
  (params (player :type "AGSDCharacter Object Reference"))
  (returns (ReturnValue :type Boolean))
  (return false))

(fn `UserConstructionScript`)