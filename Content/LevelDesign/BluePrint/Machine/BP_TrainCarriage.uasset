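; A train carriage pawn that drives itself along the spline of its active path using floating pawn movement.
; Each tick it moves forward and turns toward a look-ahead point found from the nearest spline tangent, stopping at the spline's end.
; A timeline ramps max speed up or, reversed, down.
; A farmer entering or leaving its box trigger calls train go or stop on a target reference.
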(event `self.ReceiveTick`
  (params (DeltaSeconds :type "Float (single-precision)"))
  (if (not (`self.Stop`))
    (`self.AddMovementInput` (`self.GetActorForwardVector`) (`self.Speed`))
    (`self.Get Path`)))

(event `Speed Up`
  (bind (_direction _start) (`Timeline|Start` :!label _label)
    (:`Update`
      (bind _output_get (set `FloatingPawnMovement.MaxSpeed` _start (`self.FloatingPawnMovement`)))
      (set `self.Stop` (<= _output_get 0.0)))))

(event `Slow Down`
  (goto _label :!via `Reverse`))

(event `self.Box.OnComponentBeginOverlap`
  (params (OverlappedComponent :type "PrimitiveComponent Object Reference") (OtherActor :type "Actor Object Reference") (OtherComp :type "PrimitiveComponent Object Reference") (OtherBodyIndex :type Integer) (bFromSweep :type Boolean) (SweepResult :type "HitResult Structure (by ref)"))
  (cast `/Game/HYH/Blueprints/BP_Farmer` OtherActor)
  (`/Game/LevelDesign/BluePrint/Machine/BP_Train.Train Go` (`self.Target`)))

(event `self.Box.OnComponentEndOverlap`
  (params (OverlappedComponent :type "PrimitiveComponent Object Reference") (OtherActor :type "Actor Object Reference") (OtherComp :type "PrimitiveComponent Object Reference") (OtherBodyIndex :type Integer))
  (cast `/Game/HYH/Blueprints/BP_Farmer` OtherActor)
  (`/Game/LevelDesign/BluePrint/Machine/BP_Train.Train Stop` (`self.Target`)))

(fn `Get Path`
  (bind _returnvalue (`self.K2_GetActorLocation`))
  (bind _active_path (`self.Active Path`))
  (bind _spline (`/Game/LevelDesign/BluePrint/Machine/BP_TrainTrack.Spline` _active_path))
  (`/Engine/EditorBlueprintResources/StandardMacros.IsValid` _active_path
    (:`Is Valid`
      (if (== (`SplineComponent.GetLocationAtSplinePoint` _spline (`SplineComponent.GetNumberOfSplinePoints` _spline) "World") _returnvalue :`ErrorTolerance` 50.0)
        (set `self.Stop` true)
        (else
          (`self.K2_SetActorRotation` (`KismetMathLibrary.FindLookAtRotation` _returnvalue (`SplineComponent.FindLocationClosestToWorldLocation` _spline (+ (* (`KismetMathLibrary.Normal` (`SplineComponent.FindTangentClosestToWorldLocation` _spline _returnvalue "World")) 50.0) _returnvalue) "World"))))))))

(fn `UserConstructionScript`)